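; Base character for turn-based battle entities, controlled by player or AI by team.
; Init applies mesh, animation, effects and spells from a data asset, and renders an icon via scene capture of a temporary actor.
; Move-and-cast (single-target only) feeds AI blackboard movement, then range-checks and activates the GAS ability.
; Tick charges distance travelled to the Movement attribute through a gameplay effect, halting the character when it runs out.
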(event `self.ReceiveBeginPlay`)

(event `self.ReceiveTick`
  (params (DeltaSeconds :type "Float (single-precision)"))
  (bind _returnvalue (`self.K2_GetActorLocation`))
  (if (`self.IsMoving`)
    (if (`self.MovementIsSet`)
      (set `self.CurrentLocation` (`self.K2_GetActorLocation`))
      (bind _canpay (`self.CanPayMovementCost` 0.0))
      (if _canpay
        (`self.PayMovementCost` self (`self.AbilitySystemComponent`) (`KismetMathLibrary.VSize` (- (`self.CurrentLocation`) (`self.PreviousLocation`))))
        (set `self.PreviousLocation` (`self.CurrentLocation`))
        (else
          (`MovementComponent.StopMovementImmediately` (`self.CharacterMovement`))
          (`self.SetIsMoving` false)))
      (else
        (set `self.CurrentLocation` _returnvalue)
        (set `self.PreviousLocation` _returnvalue)
        (set `self.MovementIsSet` true)))))

(event `AIStartTurn`
  (bind _returnvalue (`AIBlueprintHelperLibrary.GetBlackboard` (`self.As BP AITemplate Controllable`)))
  (if (`self.bControlledByAI`)
    (`KismetSystemLibrary.PrintString` "AI StartingTurn" true true (struct :`R` 1.0 :`G` 0.931191 :`A` 1.0))
    (`/Engine/EditorBlueprintResources/StandardMacros.IsValid` _returnvalue
      (:`Is Valid`
        (`BlackboardComponent.SetValueAsBool` _returnvalue "IsAITurn" true)
        (`KismetSystemLibrary.PrintString` "Balckboard value for starting turn is set" true true (struct :`R` 1.0 :`G` 0.869375 :`A` 1.0) 4.0))
      (:`Is Not Valid`
        (`KismetSystemLibrary.PrintString` "AI Blackboard is not valide" true true (struct :`R` 1.0 :`G` 0.931191 :`A` 1.0))))))

(event `OnTurnStart`
  (`BlackboardComponent.SetValueAsBool` (`AIBlueprintHelperLibrary.GetBlackboard` null) "IsMyTurn" true)
  (`self.HandleStartOfTurnEffect`)
  (`self.DecreaseTurnRemainingOnOverTurnEffect`))

(event `UseSpellAfterMovement`
  (bind _destination (`self.Destination`))
  (bind _spellbeingcast (`self.SpellBeingCast`))
  (bind _returnvalue (`KismetMathLibrary.FMax` (.z (`self.K2_GetActorLocation` (`self.Caster`))) (.z (`self.Destination`))))
  (`/Engine/EditorBlueprintResources/StandardMacros.IsValid` (`self.SpellBeingCast`)
    (:`Is Valid`
      (`self.K2_SetActorRotation` (`self.Caster`) (`KismetMathLibrary.MakeRotator` 0.0 0.0 (.yaw (`KismetMathLibrary.FindLookAtRotation` (`self.K2_GetActorLocation` (`self.Caster`)) (`self.Destination`)))) false)
      (bind _targets (`/Game/Blueprints/BP_BattleGameController.FindSpellTargets` (`self.As BP Battle Game Controller`) (`self.MainTarget`) _destination _spellbeingcast))
      (bind _output_get (set `self.SpellTargets` _targets))
      (`/Engine/EditorBlueprintResources/StandardMacros.IsValid` (`self.MainTarget`)
        (:`Is Valid`
          (`KismetArrayLibrary.Array_AddUnique` _output_get (`self.MainTarget`)))
        (:`Is Not Valid`
          _))
      (if (<= (`KismetMathLibrary.Vector_Distance` (`KismetMathLibrary.MakeVector` (.x (`self.K2_GetActorLocation` (`self.Caster`))) (.y (`self.K2_GetActorLocation` (`self.Caster`))) _returnvalue) (`KismetMathLibrary.MakeVector` (.x (`self.Destination`)) (.y (`self.Destination`)) _returnvalue)) (`AbilitiesDataAsset.Range` (`COTDGameplayAbility.AbilitiesDataAsset` (`self.SpellBeingCast`))))
        (`self.UseSpell` (`self.Caster`) _spellbeingcast _output_get _destination)
        (`/Game/Blueprints/BP_BattleGameController.CancelCastSpell` (`self.As BP Battle Game Controller`) true)
        (else
          (`KismetSystemLibrary.PrintText` "NOT N RANGE" true true (struct :`R` 1.0 :`A` 1.0)))))))

(event `MoveAndCastSpell`
  (params (Spell :type "COTDGameplayAbility Object Reference"))
  (bind (_bblockinghit _binitialoverlap _time _distance _location _impactpoint _normal _impactnormal _physmat _hitactor) (`GameplayStatics.BreakHitResult` (`PlayerController.GetHitResultUnderCursorByChannel` (`self.As BP Battle Game Controller`) "TraceTypeQuery1" true)))
  (`KismetSystemLibrary.PrintString` "Move and cast spell called" true true (struct :`R` 1.0 :`G` 0.42556 :`B` 0.234393 :`A` 1.0) 3.0)
  (set `self.SpellBeingCast` Spell)
  (`/Engine/EditorBlueprintResources/StandardMacros.IsValid` self
    (:`Is Valid`
      (if (`self.CanControl`)
        (set `self.CanControl` true)
        (`KismetArrayLibrary.Array_Clear` (`self.SpellTargets`))
        (set `self.MainTarget` null)
        (bind _output_get (set `self.Caster` self))
        (set `self.Destination` _location)
        (`/Engine/EditorBlueprintResources/StandardMacros.IsValid` (`self.SpellBeingCast`)
          (:`Is Valid`
            (switch `ETargetingType` (`AbilitiesDataAsset.TargetingType` (`COTDGameplayAbility.AbilitiesDataAsset` (`self.SpellBeingCast`)))
              (:`SingleTarget`
                (bind _asbp_template_controllable (cast `/Game/Blueprints/Entities/Controllable/BP_TemplateControllable` _hitactor)
                  (:`then`
                    (set `self.MainTarget` _asbp_template_controllable))
                  (:`CastFailed`
                    _))
                (`self.EventMovement` (`self.Caster`) (`self.Destination`) :!label _label))
              (:`MultiTarget`
                (`/Game/Blueprints/BP_BattleGameController.CancelCastSpell` (`self.As BP Battle Game Controller`) false :!label _label_2)
                (`KismetSystemLibrary.PrintText` "TBD"))
              (:`AreaOfEffect`
                (goto _label_2))
              (:`Self`
                (goto _label_2))
              (:`Global`
                (goto _label_2))))
          (:`Is Not Valid`
            (goto _label)))))
    (:`Is Not Valid`
      (`/Game/Blueprints/BP_BattleGameController.CancelCastSpell` (`self.As BP Battle Game Controller`) false))))

(event `EventMovement`
  (params (Destination :type "Vector Structure"))
  (bind _as_bp_aitemplate_controllable (`self.As BP AITemplate Controllable`))
  (bind _returnvalue (`AIBlueprintHelperLibrary.GetBlackboard` _as_bp_aitemplate_controllable))
  (`Controller.StopMovement` (`AIBlueprintHelperLibrary.GetAIController` _as_bp_aitemplate_controllable))
  (`BlackboardComponent.SetValueAsBool` _returnvalue "IsMoving" true)
  (`self.DefineLineOfSightBBValueForSpell` (`self.SpellBeingCast`))
  (`BlackboardComponent.SetValueAsVector` _returnvalue "TargetLocation" Destination)
  (`KismetSystemLibrary.PrintText` "Setting all param" true true (struct :`R` 1.0 :`G` 0.593245 :`A` 1.0)))

(fn `AssociateTopIcon`
  (params (WBP_TopIcon :type "/Game/UI/Battle/WBP_EntityControllableFightIcon Object Reference"))
  (set `self.Fight Icon` WBP_TopIcon))

(fn `CanPayMovementCost`
  (params (PredictedCost :type "Float (double-precision)"))
  (returns (CanPay :type Boolean))
  (return (> (`.CurrentValue` (break `GameplayAttributeData` (`ControllableEntityAttributeSet.Movement` (`self.ControllableEntityAttributeSet`)))) 0.0)))

(fn `CheckLifeStatus`
  (if (<= (`.CurrentValue` (break `GameplayAttributeData` (`ControllableEntityAttributeSet.Health` (`self.ControllableEntityAttributeSet`)))) 0.0)
    (bind _asabp_anim_template (cast `/Game/Animation/ABP_Anim_Template` (`SkeletalMeshComponent.GetAnimInstance` (`self.Mesh`)))
      (:`then`
        (`self.PlayAnimMontage` (`BlueprintMapLibrary.Map_Find` (`/Game/Animation/ABP_Anim_Template.Montages` _asabp_anim_template) "NewEnumerator4")))
      (:`CastFailed`
        _))
    (`self.OnDeath` self)))

(fn `DefineControl`
  (params (ControlledByAI :type Boolean))
  (bind _as_bp_aitemplate_controllable (`self.As BP AITemplate Controllable`))
  (bind _output_get (set `self.bControlledByAI` ControlledByAI))
  (`Controller.UnPossess` _as_bp_aitemplate_controllable)
  (`Controller.Possess` _as_bp_aitemplate_controllable self))

(fn `DefineLineOfSightBBValueForSpell`
  (params (GameplayAbility :type "COTDGameplayAbility Object Reference"))
  (bind _returnvalue (`AIBlueprintHelperLibrary.GetBlackboard` (`self.As BP AITemplate Controllable`)))
  (`/Engine/EditorBlueprintResources/StandardMacros.IsValid` GameplayAbility
    (:`Is Valid`
      (`BlackboardComponent.SetValueAsBool` _returnvalue "RequireLineOfSight" (`AbilitiesDataAsset.RequireLineOfSight` (`COTDGameplayAbility.AbilitiesDataAsset` GameplayAbility))))
    (:`Is Not Valid`
      (`BlackboardComponent.SetValueAsBool` _returnvalue "RequireLineOfSight" false))))

(fn `Generate Icon`
  (returns (Texture :type "Texture2D Object Reference"))
  (locals (ControllableEntity :type "EntityStats Object Reference") (SkeletalMesh :type "SkeletalMesh Object Reference") (IconGenerator :type "/Game/Blueprints/Pre-Render/BP_IconGenerator Object Reference") (AnimClass :type "AnimInstance Class Reference") (CreatedActor :type "SkeletalMeshActor Object Reference") (Material :type "Material Object Reference"))
  (bind _scenecapturecomponent2d (`/Game/Blueprints/Pre-Render/BP_IconGenerator.SceneCaptureComponent2D` (`local.IconGenerator`)))
  ;[0.1818 1 0] Setup
  (bind _entitystatsdataasset (`self.EntityStatsDataAsset`)
    (:`then`
      (`|ExecutionSequence`
        (:`then_0`
          (set `local.AnimClass` (`EntityStatsDataAsset.AnimClass` _entitystatsdataasset)))
        (:`then_1`
          (set `local.Material` (`EntityStatsDataAsset.MaterialTest` _entitystatsdataasset)))
        (:`then_2`
          (set `local.SkeletalMesh` (`EntityStatsDataAsset.SkeletonMesh` _entitystatsdataasset))
          (bind _returnvalue (`GameplayStatics.GetActorOfClass` "/Game/Blueprints/Pre-Render/BP_IconGenerator.BP_IconGenerator_C"))
          (set `local.IconGenerator` _returnvalue)
          (bind _returnvalue_2 (`|SpawnActorFromClass` "/Game/Blueprints/Pre-Render/BP_PreRenderControllableEntity.BP_PreRenderControllableEntity_C" (`KismetMathLibrary.MakeTransform` (.location (`SceneComponent.K2_GetComponentToWorld` (`/Game/Blueprints/Pre-Render/BP_IconGenerator.Stele` (`local.IconGenerator`)))) (struct :`Yaw` 90.0)) "Undefined" "MultiplyWithRoot" null null))
          (bind _output_get (set `local.CreatedActor` _returnvalue_2))
          (`SkeletalMeshComponent.SetSkeletalMeshAsset` (`SkeletalMeshActor.SkeletalMeshComponent` _returnvalue_2) (`local.SkeletalMesh`))
          (`PrimitiveComponent.SetMaterial` (`SkeletalMeshActor.SkeletalMeshComponent` _returnvalue_2) 0 (`local.Material`))
          (`PrimitiveComponent.SetMaterial` (`SkeletalMeshActor.SkeletalMeshComponent` _output_get) 0 (`local.Material`))
          (`SkeletalMeshComponent.SetAnimInstanceClass` (`SkeletalMeshActor.SkeletalMeshComponent` _returnvalue_2) (`local.AnimClass`))
          (`SceneCaptureComponent2D.CaptureScene` _scenecapturecomponent2d)
          (bind _returnvalue_3 (`IconGenerator.ConvertRenderTargetToTexture2D` (`local.IconGenerator`) (`SceneCaptureComponent2D.TextureTarget` _scenecapturecomponent2d)))
          (`self.K2_DestroyActor` (`local.CreatedActor`))
          (return _returnvalue_3))))
    (:`else`)))

(fn `GetHealthPercent`
  (returns (HealthRemainingPercent :type "Float (double-precision)"))
  (bind _controllableentityattributeset (`self.ControllableEntityAttributeSet`))
  (`/Engine/EditorBlueprintResources/StandardMacros.IsValid` self
    (:`Is Valid`
      (`/Engine/EditorBlueprintResources/StandardMacros.IsValid` _controllableentityattributeset
        (:`Is Valid`
          (return (- 1.0 (`KismetMathLibrary.NormalizeToRange` (`.CurrentValue` (break `GameplayAttributeData` (`ControllableEntityAttributeSet.Health` _controllableentityattributeset))) 0.0 (`.CurrentValue` (break `GameplayAttributeData` (`ControllableEntityAttributeSet.MaxHealth` _controllableentityattributeset)))))))
        (:`Is Not Valid`
          (`KismetSystemLibrary.PrintText` (`|FormatText` "Not valid forControllableAttibuteSet {obj} \n" (`KismetSystemLibrary.GetDisplayName` self)) true true (struct :`R` 1.0 :`G` 0.040611 :`A` 1.0) 5.0))))
    (:`Is Not Valid`
      (`KismetSystemLibrary.PrintText` "Not valid for BP_Controllable" true true (struct :`R` 1.0 :`G` 0.040611 :`A` 1.0) 5.0))))

(fn `HealthBarUIUpdate`
  (if (== (`/Game/Blueprints/BP_BattleGameController.SelectedControllableEntity` (`self.As BP Battle Game Controller`)) self)
    (bind _asbp_battle_game_mode (cast `/Game/Blueprints/BP_BattleGameMode` (`GameplayStatics.GetGameMode`)))
    (bind _healthremainingpercent (`self.GetHealthPercent`))
    (`ProgressBar.SetPercent` (`/Game/UI/Battle/WBP_SpellBar.EntityLifeFillBar` (`/Game/Blueprints/BP_BattleGameMode.BattleUISpellBarWidget` _asbp_battle_game_mode)) _healthremainingpercent)))

(fn `Init`
  (params (Team :type Integer64))
  (`|ExecutionSequence`
    (:`then_0`
      (bind _entitystatsdataasset (`self.EntityStatsDataAsset`)
        (:`then`
          (`|ExecutionSequence`
            (:`then_0`
              (`SkeletalMeshComponent.SetSkeletalMeshAsset` (`self.Mesh`) (`EntityStatsDataAsset.SkeletonMesh` _entitystatsdataasset))
              (`PrimitiveComponent.SetMaterial` (`self.Mesh`) 0 (`EntityStatsDataAsset.MaterialTest` _entitystatsdataasset)))
            (:`then_1`
              (`SkeletalMeshComponent.SetAnimInstanceClass` (`self.Mesh`) (`EntityStatsDataAsset.AnimClass` _entitystatsdataasset)))
            (:`then_2`
              (`self.DataTableSetup`))
            (:`then_3`
              (for _array_element (`EntityStatsDataAsset.StartingEffects` _entitystatsdataasset)
                (`AbilitySystemComponent.BP_ApplyGameplayEffectToSelf` :`self` (`self.AbilitySystemComponent`) :`GameplayEffectClass` _array_element)))))
        (:`else`)))
    (:`then_1`
      (bind _asbp_battle_game_mode (cast `/Game/Blueprints/BP_BattleGameMode` (`GameplayStatics.GetGameMode`)))
      (set `self.As BP Battle Game Mode` _asbp_battle_game_mode))
    (:`then_2`
      (bind _asbp_battle_game_controller (cast `/Game/Blueprints/BP_BattleGameController` (`GameplayStatics.GetPlayerController` 0)))
      (set `self.As BP Battle Game Controller` _asbp_battle_game_controller))
    (:`then_3`
      (bind _asbp_aitemplate_controllable (cast `/Game/Blueprints/Entities/Controllable/BP_AITemplateControllable` (`AIBlueprintHelperLibrary.GetAIController` self))
        (:`then`
          (set `self.As BP AITemplate Controllable` _asbp_aitemplate_controllable))
        (:`CastFailed`
          (`KismetSystemLibrary.PrintText` "Cast to AITemplate Failed" true true (struct :`R` 1.0 :`G` 0.007047 :`A` 1.0)))))
    (:`then_4`
      (set `self.CanControl` true))
    (:`then_5`
      (bind _texture (`self.Generate Icon`))
      (set `self.UncutIcon` _texture))
    (:`then_6`
      (`self.SetupSpell`))
    (:`then_8`
      (set `self.IsInit` true))
    (:`then_9`
      (bind _output_get (set `self.Team` Team))
      (`self.DefineControl` (!= _output_get 0)))
    (:`then_10`
      (`KismetSystemLibrary.PrintText` (`KismetTextLibrary.Conv_ObjectToText` (`AIBlueprintHelperLibrary.GetAIController` self)) true true (struct :`R` 1.0 :`G` 0.799144 :`A` 1.0) 6.0))))

(fn `PayMovementCost`
  (params (ASC :type "AbilitySystemComponent Object Reference") (MovementCost :type "Float (double-precision)"))
  (bind _returnvalue (`AbilitySystemBlueprintLibrary.MakeSpecHandleByClass` "/Game/GE_GameplayEffect/GE_PayMovement.GE_PayMovement_C"))
  (bind _returnvalue_2 (`AbilitySystemBlueprintLibrary.AssignTagSetByCallerMagnitude` _returnvalue (struct :`TagName` "Ressources.Movement") (* (`KismetMathLibrary.Abs` MovementCost) -1.0)))
  (`AbilitySystemComponent.BP_ApplyGameplayEffectSpecToSelf` ASC _returnvalue_2)
  (if (== (`/Game/Blueprints/BP_BattleGameController.SelectedControllableEntity` (`self.As BP Battle Game Controller`)) self)
    (`/Game/UI/Battle/WBP_SpellBar.RefreshPanelInfo` (`/Game/Blueprints/BP_BattleGameMode.BattleUISpellBarWidget` (`self.As BP Battle Game Mode`)) self)))

(fn `SetIsMoving`
  (params (IsMoving :type Boolean))
  (set `self.IsMoving` IsMoving)
  (set `self.MovementIsSet` false))

(fn `SetupSpell`
  (for _array_element (`EntityStatsDataAsset.EntitySpells` (`self.EntityStatsDataAsset`))
    (`AbilitySystemComponent.K2_GiveAbility` (`self.AbilitySystemComponent`) _array_element 0 -1)))

(fn `UserConstructionScript`)

(fn `UseSpell`
  (params (SpellToUse :type "COTDGameplayAbility Object Reference") (SpellTargets :type "Array of /Game/Blueprints/Entities/Controllable/BP_TemplateControllable Object Reference") (SpellUseLocation :type "Vector Structure"))
  (`KismetArrayLibrary.Array_Clear` (`self.SpellsTargetCopy`))
  (set `self.SpellsTargetCopy` SpellTargets)
  (`/Engine/EditorBlueprintResources/StandardMacros.IsValid` SpellToUse
    (:`Is Valid`
      (set `self.SpellBeingCast` SpellToUse)
      (set `self.SpellLocation` SpellUseLocation)
      (`AbilitySystemComponent.TryActivateAbilityByClass` (`self.AbilitySystemComponent`) (`GameplayStatics.GetObjectClass` SpellToUse) true))
    (:`Is Not Valid`
      (`KismetArrayLibrary.Array_Clear` (`self.SpellsTargetCopy`)))))