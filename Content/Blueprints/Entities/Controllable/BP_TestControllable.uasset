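; BP_TestControllable is a test controllable entity whose appearance comes from an EntityStatsDataAsset.
; When that asset is valid, the construction script applies its skeletal mesh, test material and animation class to the Mesh.
; On BeginPlay it issues a single AI move to a random reachable navigation point within a large radius of its location.
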(event `self.ReceiveBeginPlay`
  (`|AIMoveTo` self (`NavigationSystemV1.K2_GetRandomReachablePointInRadius` (`self.K2_GetActorLocation` self) 10000.0 null null) null))

(fn `UserConstructionScript`
  (bind _entitystatsdataasset (`self.EntityStatsDataAsset`)
    (:`then`
      (`|ExecutionSequence`
        (:`then_0`
          (`SkeletalMeshComponent.SetSkeletalMeshAsset` (`self.Mesh`) (`EntityStatsDataAsset.SkeletonMesh` _entitystatsdataasset))
          (`PrimitiveComponent.SetMaterial` (`self.Mesh`) 0 (`EntityStatsDataAsset.MaterialTest` _entitystatsdataasset)))
        (:`then_1`
          (`SkeletalMeshComponent.SetAnimInstanceClass` (`self.Mesh`) (`EntityStatsDataAsset.AnimClass` _entitystatsdataasset)))))
    (:`else`)))