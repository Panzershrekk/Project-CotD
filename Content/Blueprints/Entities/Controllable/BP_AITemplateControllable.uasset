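; Template AI controller for controllable entities that starts their AI when it possesses a pawn.
; On possession, it runs the BT_Entity behavior tree through the possessed pawn's AI controller.
; It then checks the blackboard and prints color-coded debug text showing the possession, whether the blackboard is valid and, if so, the result of starting the tree.
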(event `self.ReceivePossess`
  (params (PossessedPawn :type "Pawn Object Reference"))
  (bind _returnvalue (`AIBlueprintHelperLibrary.GetBlackboard` null))
  (`KismetSystemLibrary.PrintText` (`|FormatText` "Possesed {Possesed}" (`KismetSystemLibrary.GetObjectName` self)) true true (struct :`R` 0.316971 :`G` 1.0 :`B` 0.171417 :`A` 1.0) 6.0)
  (bind _returnvalue_2 (`self.RunBehaviorTree` (`AIBlueprintHelperLibrary.GetAIController` PossessedPawn) "/Game/Blueprints/Entities/Controllable/EQS/BT_Entity.BT_Entity"))
  (`/Engine/EditorBlueprintResources/StandardMacros.IsValid` _returnvalue
    (:`Is Valid`
      (`KismetSystemLibrary.PrintText` (`|FormatText` "Blackboard {bbname} is valid, running state is {state}" (`KismetSystemLibrary.GetPathName` _returnvalue) _returnvalue_2) true true (struct :`R` 0.1305 :`G` 1.0 :`B` 0.063542 :`A` 1.0) 4.0))
    (:`Is Not Valid`
      (`KismetSystemLibrary.PrintText` (`|FormatText` "Blackboard {bbname} is not valid" _returnvalue) true true (struct :`R` 1.0 :`A` 1.0) 4.0))))

(fn `UserConstructionScript`)