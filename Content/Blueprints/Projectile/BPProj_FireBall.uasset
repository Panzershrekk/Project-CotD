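; BPProj_FireBall is a fireball projectile Blueprint that adds a fire trail effect on top of its parent class.
; On BeginPlay it spawns the FireTrail particle system attached to the Sphere component with auto-destroy and stores it in Particle.
; A Test event deactivates that trail, while overlap handling and construction only call the parent implementations.
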(event `self.ReceiveBeginPlay`
  (bind _returnvalue (`NiagaraFunctionLibrary.SpawnSystemAttached` "/Game/FX/FireTrail.FireTrail" (`self.Sphere`) "None" (0.0 0.0 0.0) (struct) "KeepRelativeOffset" true))
  (set `self.Particle` _returnvalue))

(event `self.ReceiveActorBeginOverlap`
  (params (OtherActor :type "Actor Object Reference"))
  (`parent.ReceiveActorBeginOverlap` OtherActor))

(event `self.Test`
  (`ActorComponent.Deactivate` (`self.Particle`)))

(fn `UserConstructionScript`
  (`parent.UserConstructionScript`))