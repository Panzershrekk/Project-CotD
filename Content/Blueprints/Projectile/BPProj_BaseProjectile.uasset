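; Base spell projectile that flies in a straight line to a target point and ends in a fire explosion.
; Setup stores the spell, speed and destination and enables movement, which Tick performs by setting the actor location without sweep or overlap handling.
; Near the destination it calls OnFinished, spawns a Niagara explosion sized from the spell data asset's area selector radius, then destroys itself.
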(event `self.ReceiveTick`
  (params (DeltaSeconds :type "Float (single-precision)"))
  (bind _returnvalue (`self.K2_GetActorLocation`))
  (bind _returnvalue_2 (+ _returnvalue (* (`KismetMathLibrary.Normal` (- (`self.Destination`) _returnvalue)) DeltaSeconds (`self.Speed`))))
  (if (`self.CanMove`)
    (`self.K2_SetActorLocation` _returnvalue_2)
    (if (<= (`KismetMathLibrary.Vector_Distance` (`self.Destination`) _returnvalue_2) 50.0)
      (`self.OnFinished`)
      (bind _returnvalue_3 (`NiagaraFunctionLibrary.SpawnSystemAtLocation` "/Game/FX/FireExplosion.FireExplosion" (`self.K2_GetActorLocation`)))
      (`NiagaraComponent.SetVariableFloat` _returnvalue_3 "Radius" (`AbilitiesDataAsset.AreaSelectorRadius` (`COTDGameplayAbility.AbilitiesDataAsset` (`self.Spell`))))
      (`self.K2_DestroyActor`))))

(fn `Setup`
  (params (Spell :type "COTDGameplayAbility Object Reference") (ParamSpeed :type "Float (double-precision)") (ParamDestination :type "Vector Structure"))
  (set `self.Spell` Spell)
  (set `self.Speed` ParamSpeed)
  (set `self.Destination` ParamDestination)
  (set `self.CanMove` true))

(fn `UserConstructionScript`)