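; BP_SphereHitbox is a spherical spell hitbox that tracks and highlights the BP_TemplateControllable actors inside it.
; Sphere begin and end overlap events add or remove actors in EntityOverlapped and toggle each mesh's custom depth and stencil value.
; ClearOverlapped resets that highlight and removes entries, but does so while iterating the same array, so it can skip elements.
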(event `self.HitboxSphere.OnComponentBeginOverlap`
  (params (OverlappedComponent :type "PrimitiveComponent Object Reference") (OtherActor :type "Actor Object Reference") (OtherComp :type "PrimitiveComponent Object Reference") (OtherBodyIndex :type Integer) (bFromSweep :type Boolean) (SweepResult :type "HitResult Structure (by ref)"))
  (bind _asbp_template_controllable (cast `/Game/Blueprints/Entities/Controllable/BP_TemplateControllable` OtherActor))
  (`KismetArrayLibrary.Array_Add` (`self.EntityOverlapped`) _asbp_template_controllable)
  (bind _mesh (`Character.Mesh` _asbp_template_controllable))
  (`PrimitiveComponent.SetRenderCustomDepth` _mesh true)
  (`PrimitiveComponent.SetCustomDepthStencilValue` _mesh 1))

(event `self.HitboxSphere.OnComponentEndOverlap`
  (params (OverlappedComponent :type "PrimitiveComponent Object Reference") (OtherActor :type "Actor Object Reference") (OtherComp :type "PrimitiveComponent Object Reference") (OtherBodyIndex :type Integer))
  (bind _asbp_template_controllable (cast `/Game/Blueprints/Entities/Controllable/BP_TemplateControllable` OtherActor))
  (`KismetArrayLibrary.Array_RemoveItem` (`self.EntityOverlapped`) _asbp_template_controllable)
  (bind _mesh (`Character.Mesh` _asbp_template_controllable))
  (`PrimitiveComponent.SetRenderCustomDepth` _mesh false)
  (`PrimitiveComponent.SetCustomDepthStencilValue` _mesh 0))

(fn `ClearOverlapped`
  (for _array_element (`self.EntityOverlapped`)
    (`KismetArrayLibrary.Array_RemoveItem` (`self.EntityOverlapped`) _array_element)
    (bind _mesh (`Character.Mesh` _array_element))
    (`PrimitiveComponent.SetRenderCustomDepth` _mesh false)
    (`PrimitiveComponent.SetCustomDepthStencilValue` _mesh 0)))

(fn `UserConstructionScript`)