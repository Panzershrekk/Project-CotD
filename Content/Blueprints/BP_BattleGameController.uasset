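; Player controller for turn-based battles, handling the pan/zoom battle camera, entity selection, click-to-move, right-click examine and spell casting.
; SetControllableEntity fills the game mode's spell bar; InitCastSpell shows a cursor icon, range decal and area selector that snaps to hovered entities.
; MoveAndCastSpell walks the caster into range via AIMoveTo, then gathers area victims with a temporary sphere hitbox.
; Only single-target targeting is implemented; other types cancel.
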(event `Setup`
  (params (GameMode :type "/Game/Blueprints/BP_BattleGameMode Object Reference"))
  (set `self. BPBattlegameMode` GameMode)
  (`|ExecutionSequence`
    (:`then_0`
      (set `self.bShowMouseCursor` true))
    (:`then_1`
      (bind _outactors (`GameplayStatics.GetAllActorsOfClass` "/Game/Blueprints/BP_BattleCamera.BP_BattleCamera_C"))
      (bind _output_get (set `self.CameraActor` (`|GetArrayItem` _outactors)))
      (`self.SetViewTargetWithBlend` (`GameplayStatics.GetPlayerController` 0) _output_get 0.0 "VTBlend_Linear" 0.0 false)
      (bind _cameraactor (`self.CameraActor`)
        (:`then`
          (`self.K2_SetActorLocation` _cameraactor (`self.K2_GetActorLocation` (`self.CameraActor`)) false true))
        (:`else`)))
    (:`then_2`
      (bind _returnvalue (`|CreateWidget` "/Game/UI/Battle/WBP_Spell.WBP_Spell_C" null "/Game/Image/SimpleCadre.SimpleCadre"))
      (bind _output_get_2 (set `self.SpellIconFollowingMouse` _returnvalue))
      (`UserWidget.AddToViewport` _output_get_2 0)
      (`Widget.SetVisibility` _output_get_2 "Hidden"))
    (:`then_3`
      (`self.PrepareTargetSelector`))))

(event `Key|MouseScrollUp`
  (params (Key :type "Key Structure"))
  (:`Pressed`
    (set `SpringArmComponent.TargetArmLength` (`KismetMathLibrary.FClamp` (+ (`SpringArmComponent.TargetArmLength` (`/Game/Blueprints/BP_BattleCamera.SpringArm` (`self.CameraActor`))) -50.0) 100.0 2000.0) (`/Game/Blueprints/BP_BattleCamera.SpringArm` (`self.CameraActor`)))))

(event `Key|MouseScrollDown`
  (params (Key :type "Key Structure"))
  (:`Pressed`
    (set `SpringArmComponent.TargetArmLength` (`KismetMathLibrary.FClamp` (+ (`SpringArmComponent.TargetArmLength` (`/Game/Blueprints/BP_BattleCamera.SpringArm` (`self.CameraActor`))) 50.0) 100.0 2000.0) (`/Game/Blueprints/BP_BattleCamera.SpringArm` (`self.CameraActor`)))))

(event `InputAxis|MoveForward`
  (params (AxisValue :type "Float (single-precision)"))
  (bind _cameraactor (`self.CameraActor`))
  (`/Engine/EditorBlueprintResources/StandardMacros.IsValid` _cameraactor
    (:`Is Valid`
      (`self.K2_AddActorLocalOffset` _cameraactor (`KismetMathLibrary.MakeVector` (* AxisValue (`GameplayStatics.GetWorldDeltaSeconds`) (`self.CameraSpeed`))) false false))))

(event `InputAxis|MoveLateral`
  (params (AxisValue :type "Float (single-precision)"))
  (bind _cameraactor (`self.CameraActor`))
  (`/Engine/EditorBlueprintResources/StandardMacros.IsValid` _cameraactor
    (:`Is Valid`
      (`self.K2_AddActorLocalOffset` _cameraactor (`KismetMathLibrary.MakeVector` 0.0 (* AxisValue (`GameplayStatics.GetWorldDeltaSeconds`) (`self.CameraSpeed`))) false false))))

(event `self.ReceiveTick`
  (params (DeltaSeconds :type "Float (single-precision)"))
  (bind (_locationx _locationy _returnvalue) (`self.GetMousePosition`))
  (bind _targetsphereselector (`self.TargetSphereSelector`))
  (bind (_bblockinghit _binitialoverlap _time _distance _location _impactpoint _normal _impactnormal _physmat _hitactor) (`GameplayStatics.BreakHitResult` (`self.GetHitResultUnderCursorByChannel` "TraceTypeQuery1")))
  ;[1 0.6986 0] Outline
  (`|ExecutionSequence`
    (:`then_0`
      (if (`self.SpellIsBeingCast`)
        (`|ExecutionSequence`
          (:`then_0`
            (if _returnvalue
              (`UserWidget.SetPositionInViewport` (`self.SpellIconFollowingMouse`) (`KismetMathLibrary.MakeVector2D` _locationx _locationy) true))))))
    (:`then_1`
      (`/Engine/EditorBlueprintResources/StandardMacros.IsValid` _targetsphereselector
        (:`Is Valid`
          (bind _asbp_template_controllable (cast `/Game/Blueprints/Entities/Controllable/BP_TemplateControllable` _hitactor)
            (:`then`
              ;;[1 0.2314 0.06127] Snap to target
              (`self.K2_SetActorLocation` _targetsphereselector (`self.K2_GetActorLocation` _asbp_template_controllable) false false))
            (:`CastFailed`
              (`self.K2_SetActorLocation` _targetsphereselector _location false false))))))))

(event `Key|LeftMouseButton`
  (params (Key :type "Key Structure"))
  (bind _selectedcontrollableentity (`self.SelectedControllableEntity`))
  (:`Pressed`
    (if (`self.SpellIsBeingCast`)
      (`self.MoveAndCastSpell`)
      (else
        ;[0.3073 0.1316 0] Getting a Controllable entity by left click
        (`/Engine/EditorBlueprintResources/StandardMacros.IsValid` _selectedcontrollableentity
          (:`Is Valid`
            (if (`/Game/Blueprints/Entities/Controllable/BP_TemplateControllable.bControlledByAI` _selectedcontrollableentity)
              _
              (elif (`/Game/Blueprints/Entities/Controllable/BP_TemplateControllable.CanControl` _selectedcontrollableentity)
                (if (`/Game/Blueprints/Entities/Controllable/BP_TemplateControllable.IsHisTurn` _selectedcontrollableentity)
                  ;[1 0 0.1145] MovingEntityToMouseClick
                  (`|AIMoveTo` (`self.SelectedControllableEntity`) (`.Location` (`GameplayStatics.BreakHitResult` (`self.GetHitResultUnderCursorByChannel` "TraceTypeQuery1"))) null 10.0)))))
          (:`Is Not Valid`
            (`self.SelectControllableEntity`)))))))

(event `Key|RightMouseButton`
  (params (Key :type "Key Structure"))
  ;[1 0 0] Removing Info on right mouse click
  (:`Pressed`
    (`self.CancelAction`)
    (bind _asbp_template_controllable (cast `/Game/Blueprints/Entities/Controllable/BP_TemplateControllable` (`.HitActor` (`GameplayStatics.BreakHitResult` (`self.GetHitResultUnderCursorByChannel` "TraceTypeQuery1")))))
    (`/Game/UI/Battle/WBP_Examine.ChargeInformationAndShow` (`/Game/Blueprints/BP_BattleGameMode.BattleUIExamine` (`self. BPBattlegameMode`)) _asbp_template_controllable)))

(event `MoveAndCastSpell`
  (bind _destination (`self.Destination`))
  (bind _spellbeingcast (`self.SpellBeingCast`))
  (bind _selectedcontrollableentity (`self.SelectedControllableEntity`))
  (bind (_bblockinghit _binitialoverlap _time _distance _location _impactpoint _normal _impactnormal _physmat _hitactor) (`GameplayStatics.BreakHitResult` (`self.GetHitResultUnderCursorByChannel` "TraceTypeQuery1")))
  (bind _range (`AbilitiesDataAsset.Range` (`COTDGameplayAbility.AbilitiesDataAsset` _spellbeingcast)))
  (`/Engine/EditorBlueprintResources/StandardMacros.IsValid` _selectedcontrollableentity
    (:`Is Valid`
      (if (`/Game/Blueprints/Entities/Controllable/BP_TemplateControllable.CanControl` _selectedcontrollableentity)
        (set `/Game/Blueprints/Entities/Controllable/BP_TemplateControllable.CanControl` false _selectedcontrollableentity)
        (`KismetArrayLibrary.Array_Clear` (`self.SpellTargets`))
        (set `self.MainTarget` null)
        (bind _output_get (set `self.Caster` _selectedcontrollableentity))
        (set `self.Destination` _location)
        (switch `ETargetingType` (`AbilitiesDataAsset.TargetingType` (`COTDGameplayAbility.AbilitiesDataAsset` (`self.SpellBeingCast`)))
          (:`SingleTarget`
            (bind _asbp_template_controllable (cast `/Game/Blueprints/Entities/Controllable/BP_TemplateControllable` _hitactor)
              (:`then`
                (`KismetArrayLibrary.Array_AddUnique` (`self.SpellTargets`) _asbp_template_controllable)
                (set `self.MainTarget` (`|GetArrayItem` (`self.SpellTargets`)))
                (if (<= (`self.GetHorizontalDistanceTo` (`self.Caster`) (`self.MainTarget`)) _range)
                  (`self.K2_SetActorRotation` (`self.Caster`) (`KismetMathLibrary.MakeRotator` 0.0 0.0 (.yaw (`KismetMathLibrary.FindLookAtRotation` (`self.K2_GetActorLocation` (`self.Caster`)) (`self.Destination`)))) false :!label _label)
                  (`self.FindSpellTargets` (`self.MainTarget`) _destination)
                  (`/Game/Blueprints/Entities/Controllable/BP_TemplateControllable.UseSpell` (`self.Caster`) _spellbeingcast (`self.SpellTargets`) _destination)
                  (`self.CancelCastSpell` true)
                  (else
                    (`|AIMoveTo` (`self.Caster`) (`self.Destination`) null _range :!label _label_2
                      (:`OnSuccess`
                        (goto _label))
                      (:`OnFail`
                        (`self.CancelCastSpell` false))))))
              (:`CastFailed`
                (goto _label_2))))
          (:`MultiTarget`
            (`self.CancelCastSpell` false :!label _label_3)
            (`KismetSystemLibrary.PrintText` "TBD"))
          (:`AreaOfEffect`
            (goto _label_3))
          (:`Self`
            (goto _label_3))
          (:`Global`
            (goto _label_3)))))
    (:`Is Not Valid`
      (`self.CancelCastSpell` false))))

(fn `CancelAction`
  (`|ExecutionSequence`
    (:`then_1`
      (if (`self.SpellIsBeingCast`)
        (`self.CancelCastSpell` true)))))

(fn `CancelCastSpell`
  (params (Success :type Boolean))
  (`/Game/Blueprints/BP_BattleGameMode.RefreshSpellBarUI` (`self. BPBattlegameMode`) (`self.SelectedControllableEntity`))
  (`Widget.SetVisibility` (`self.SpellIconFollowingMouse`) "Hidden")
  (`KismetArrayLibrary.Array_Clear` (`self.SpellTargets`))
  (bind _selectedcontrollableentity (`self.SelectedControllableEntity`)
    (:`then`
      (set `/Game/Blueprints/Entities/Controllable/BP_TemplateControllable.CanControl` (not Success) _selectedcontrollableentity))
    (:`else`
      _))
  (set `self.SpellIsBeingCast` false)
  (set `self.SpellBeingCast` null)
  (bind _rangedecal (`self.RangeDecal`)
    (:`then`
      (`ActorComponent.K2_DestroyComponent` _rangedecal)
      (`self.DisplaySelectorRange` false)
      (`KismetSystemLibrary.PrintString` "Canceling spell"))
    (:`else`)))

(fn `CenterCameraOnEntity`
  (params (Entity :type "/Game/Blueprints/Entities/Controllable/BP_TemplateControllable Object Reference"))
  (bind _cameraactor (`self.CameraActor`)
    (:`then`
      (`self.K2_SetActorLocation` _cameraactor (`KismetMathLibrary.MakeVector` (.x (`self.K2_GetActorLocation` Entity)) (.y (`self.K2_GetActorLocation` Entity)) (.z (`self.K2_GetActorLocation` (`self.CameraActor`)))) false false))
    (:`else`)))

(fn `DisplaySelectorRange`
  (params (IsDisplayed :type Boolean) (Range :type "Float (double-precision)" :default 1.0))
  (`SceneComponent.SetVisibility` (`self.TargetSelectorDecal`) IsDisplayed false)
  (`SphereComponent.SetSphereRadius` (`/Game/Blueprints/OutlineSelector/BP_SphereSelector.OverlappingSphere` (`self.TargetSphereSelector`)) Range true)
  ;[1 0 0.997] Need to find a way to change decal size cleanly
  (`SceneComponent.SetRelativeScale3D` (`self.TargetSelectorDecal`) (`KismetMathLibrary.MakeVector` Range Range Range)))

(fn `EndSpell`)

(fn `FindSpellTargets`
  (params (MainTarget :type "/Game/Blueprints/Entities/Controllable/BP_TemplateControllable Object Reference") (Location :type "Vector Structure"))
  (locals (TargetLocation :type "Vector Structure" :default (0.0 0.0 0.0)))
  (bind _abilitiesdataasset (`COTDGameplayAbility.AbilitiesDataAsset` (`self.SpellBeingCast`)))
  (`/Engine/EditorBlueprintResources/StandardMacros.IsValid` MainTarget
    (:`Is Valid`
      (`KismetArrayLibrary.Array_AddUnique` (`self.SpellTargets`) MainTarget)
      (if (`AbilitiesDataAsset.IsAreaOfEffect` _abilitiesdataasset)
        (set `local.TargetLocation` (`self.K2_GetActorLocation` MainTarget))
        (bind _returnvalue (`|SpawnActorFromClass` "/Game/Blueprints/SpellHitboxes/BP_SphereHitbox.BP_SphereHitbox_C" (`KismetMathLibrary.MakeTransform` (`local.TargetLocation`)) "Undefined" "MultiplyWithRoot" null null :!label _label))
        (`SphereComponent.SetSphereRadius` (`/Game/Blueprints/SpellHitboxes/BP_SphereHitbox.HitboxSphere` _returnvalue) (`AbilitiesDataAsset.AreaSelectorRadius` _abilitiesdataasset) true)
        (for _array_element (`/Game/Blueprints/SpellHitboxes/BP_SphereHitbox.EntityOverlapped` _returnvalue)
          (`KismetArrayLibrary.Array_AddUnique` (`self.SpellTargets`) _array_element))
        (`self.K2_DestroyActor` _returnvalue)))
    (:`Is Not Valid`
      (set `local.TargetLocation` Location)
      (goto _label))))

(fn `InitCastSpell`
  (params (Spell :type "COTDGameplayAbility Object Reference"))
  (bind (_locationx _locationy _returnvalue) (`self.GetMousePosition`))
  (bind _abilitiesdataasset (`COTDGameplayAbility.AbilitiesDataAsset` Spell))
  (bind _spelliconfollowingmouse (`self.SpellIconFollowingMouse`))
  (bind _range (`AbilitiesDataAsset.Range` _abilitiesdataasset))
  (`self.CancelCastSpell` false)
  (if (`/Game/Blueprints/Entities/Controllable/BP_TemplateControllable.IsHisTurn` (`self.SelectedControllableEntity`))
    (`self.SelectedControllableEntity`
      (:`then`
        (if (`/Game/Blueprints/Entities/Controllable/BP_TemplateControllable.CanControl` (`self.SelectedControllableEntity`))
          (if _returnvalue
            (`UserWidget.SetPositionInViewport` _spelliconfollowingmouse (`KismetMathLibrary.MakeVector2D` _locationx _locationy) true)
            (set `/Game/UI/Battle/WBP_Spell.SpellIcon` (`AbilitiesDataAsset.Icon` (`COTDGameplayAbility.AbilitiesDataAsset` Spell)) _spelliconfollowingmouse)
            (`Widget.SetVisibility` _spelliconfollowingmouse "Visible")
            (set `self.SpellIsBeingCast` true)
            (set `self.SpellBeingCast` Spell)
            (bind _returnvalue_2 (`GameplayStatics.SpawnDecalAtLocation` "/Game/Material/DecalMat.DecalMat" (`KismetMathLibrary.MakeVector` 5000.0 _range _range)))
            (bind _output_get (set `self.RangeDecal` _returnvalue_2))
            (`SceneComponent.K2_AttachToComponent` _output_get (`Actor.RootComponent` (`self.SelectedControllableEntity`)) "None" "KeepRelative" "KeepRelative" "KeepRelative" true)
            (if (`AbilitiesDataAsset.IsAreaOfEffect` _abilitiesdataasset)
              (`self.DisplaySelectorRange` true (`AbilitiesDataAsset.AreaSelectorRadius` _abilitiesdataasset))))
          (else
            (return))))
      (:`else`))))

(fn `PrepareTargetSelector`
  (bind _returnvalue (`|SpawnActorFromClass` "/Game/Blueprints/OutlineSelector/BP_SphereSelector.BP_SphereSelector_C" (`KismetMathLibrary.MakeTransform` (`.Location` (`GameplayStatics.BreakHitResult` (`self.GetHitResultUnderCursorByChannel` "TraceTypeQuery1")))) "Undefined" "MultiplyWithRoot" null null))
  (bind _output_get (set `self.TargetSphereSelector` _returnvalue))
  (`SphereComponent.SetSphereRadius` (`/Game/Blueprints/OutlineSelector/BP_SphereSelector.OverlappingSphere` _output_get) 1.0 true)
  (bind _returnvalue_2 (`GameplayStatics.SpawnDecalAtLocation` "/Game/Material/DecalMat.DecalMat" (`KismetMathLibrary.MakeVector` 5000.0 1.0 1.0)))
  (bind _output_get_2 (set `self.TargetSelectorDecal` _returnvalue_2))
  (`SceneComponent.K2_AttachToComponent` _output_get_2 (`Actor.RootComponent` (`self.TargetSphereSelector`)) "None" "KeepRelative" "KeepRelative" "KeepRelative" true)
  (`self.DisplaySelectorRange` false))

(fn `SelectControllableEntity`
  ;[0.3073 0.1316 0] Getting a Controllable entity by left click
  (bind _asbp_template_controllable (cast `/Game/Blueprints/Entities/Controllable/BP_TemplateControllable` (`.HitActor` (`GameplayStatics.BreakHitResult` (`self.GetHitResultUnderCursorByChannel` "TraceTypeQuery1")))))
  (`self.SetControllableEntity` _asbp_template_controllable))

(fn `SetControllableEntity`
  (params (BP_Control :type "/Game/Blueprints/Entities/Controllable/BP_TemplateControllable Object Reference"))
  (bind _selectedcontrollableentity (`self.SelectedControllableEntity`))
  (bind __bpbattlegamemode (`self. BPBattlegameMode`))
  (bind _battleuispellbarwidget (`/Game/Blueprints/BP_BattleGameMode.BattleUISpellBarWidget` __bpbattlegamemode))
  (`/Engine/EditorBlueprintResources/StandardMacros.IsValid` BP_Control
    (:`Is Valid`
      (`/Engine/EditorBlueprintResources/StandardMacros.IsValid` __bpbattlegamemode
        (:`Is Valid`
          (bind _output_get (set `self.SelectedControllableEntity` BP_Control))
          (`/Engine/EditorBlueprintResources/StandardMacros.IsValid` _battleuispellbarwidget
            (:`Is Valid`
              (`/Game/Blueprints/Entities/Controllable/BP_TemplateControllable.HealthBarUIUpdate` _output_get)
              (`Widget.SetVisibility` _battleuispellbarwidget "SelfHitTestInvisible")
              (`Image.SetBrushFromTexture` (`/Game/UI/Battle/WBP_SpellBar.EntityIcon` _battleuispellbarwidget) (`/Game/Blueprints/Entities/Controllable/BP_TemplateControllable.UncutIcon` _output_get) false)
              (`Widget.SetIsEnabled` _battleuispellbarwidget (and (`/Game/Blueprints/Entities/Controllable/BP_TemplateControllable.IsHisTurn` _selectedcontrollableentity) (!= (`/Game/Blueprints/Entities/Controllable/BP_TemplateControllable.bControlledByAI` _selectedcontrollableentity) true)))
              (`/Game/UI/Battle/WBP_SpellBar.CleanAll` _battleuispellbarwidget)
              (bind _returnvalue (`EntityStatsDataAsset.GetAbilitiesDataAssets` (`ControllableEntity.EntityStatsDataAsset` _output_get)))
              (for (_ _array_index) _returnvalue
                (bind _output (`|GetArrayItem` _returnvalue _array_index))
                (bind _output_2 (`|GetArrayItem` (`/Game/UI/Battle/WBP_SpellBar.SpellBarArray` _battleuispellbarwidget) _array_index))
                (set `/Game/UI/Battle/WBP_Spell.SpellIcon` (`AbilitiesDataAsset.Icon` (`COTDGameplayAbility.AbilitiesDataAsset` _output)) _output_2)
                (set `/Game/UI/Battle/WBP_Spell.SpellReference` _output _output_2)
                (`/Game/Blueprints/BP_BattleGameMode.RefreshSpellBarUI` (`self. BPBattlegameMode`) (`self.SelectedControllableEntity`))))
            (:`Is Not Valid`
              (`KismetSystemLibrary.PrintText` "Widget mode is not valid" true true (struct :`R` 1.0 :`A` 1.0) 10.0))))
        (:`Is Not Valid`
          (`KismetSystemLibrary.PrintText` "Geme mode is not valid" true true (struct :`R` 1.0 :`A` 1.0) 10.0))))
    (:`Is Not Valid`
      (`KismetSystemLibrary.PrintText` "Controller is not valid" true true (struct :`R` 1.0 :`A` 1.0) 10.0))))

(fn `UserConstructionScript`)