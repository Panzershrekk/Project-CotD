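; Base target zone selector actor that outlines controllable entities inside its mesh and projects the zone as a decal.
; Mesh overlaps track BP_TemplateControllable actors in EntityOverlapped and toggle their custom depth stencil, which ClearOverlapped resets.
; SetupSelectorDecal scales decal and mesh, then points an orthographic scene capture of only this actor at a bounds-sized render target feeding the decal's dynamic material.
; The construction script's copy of this setup is disconnected.
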(event `self.StaticMesh.OnComponentBeginOverlap`
  (params (OverlappedComponent :type "PrimitiveComponent Object Reference") (OtherActor :type "Actor Object Reference") (OtherComp :type "PrimitiveComponent Object Reference") (OtherBodyIndex :type Integer) (bFromSweep :type Boolean) (SweepResult :type "HitResult Structure (by ref)"))
  (bind _asbp_template_controllable (cast `/Game/Blueprints/Entities/Controllable/BP_TemplateControllable` OtherActor))
  (`KismetArrayLibrary.Array_Add` (`self.EntityOverlapped`) _asbp_template_controllable)
  (bind _mesh (`Character.Mesh` _asbp_template_controllable))
  (`PrimitiveComponent.SetRenderCustomDepth` _mesh true)
  (`PrimitiveComponent.SetCustomDepthStencilValue` _mesh 1))

(event `self.StaticMesh.OnComponentEndOverlap`
  (params (OverlappedComponent :type "PrimitiveComponent Object Reference") (OtherActor :type "Actor Object Reference") (OtherComp :type "PrimitiveComponent Object Reference") (OtherBodyIndex :type Integer))
  (bind _asbp_template_controllable (cast `/Game/Blueprints/Entities/Controllable/BP_TemplateControllable` OtherActor))
  (`KismetArrayLibrary.Array_RemoveItem` (`self.EntityOverlapped`) _asbp_template_controllable)
  (bind _mesh (`Character.Mesh` _asbp_template_controllable))
  (`PrimitiveComponent.SetRenderCustomDepth` _mesh false)
  (`PrimitiveComponent.SetCustomDepthStencilValue` _mesh 0))

(fn `ClearOverlapped`
  (for _array_element (`self.EntityOverlapped`)
    (`KismetArrayLibrary.Array_RemoveItem` (`self.EntityOverlapped`) _array_element)
    (bind _mesh (`Character.Mesh` _array_element))
    (`PrimitiveComponent.SetRenderCustomDepth` _mesh false)
    (`PrimitiveComponent.SetCustomDepthStencilValue` _mesh 0)))

(fn `SetupSelectorDecal`
  (params (XScale :type "Float (double-precision)") (YScale :type "Float (double-precision)") (Height :type "Float (double-precision)"))
  (bind _decal (`self.Decal`))
  (bind _scenecapturecomponent2d (`self.SceneCaptureComponent2D`))
  (bind (_origin _boxextent) (`KismetSystemLibrary.GetComponentBounds` (`self.StaticMesh`)))
  (bind _returnvalue (`KismetMathLibrary.FMax` (.x _boxextent) (.y _boxextent)))
  (`DecalsUtils.SetDecalSize` _decal (`KismetMathLibrary.MakeVector` (.x _boxextent) (.y _boxextent) _returnvalue))
  (`SceneComponent.SetWorldScale3D` _decal (`KismetMathLibrary.MakeVector` XScale Height YScale))
  (`SceneComponent.SetWorldScale3D` (`self.StaticMesh`) (`KismetMathLibrary.MakeVector` XScale Height YScale))
  (set `SceneCaptureComponent2D.OrthoWidth` (* _returnvalue 2.0) (`self.SceneCaptureComponent2D`))
  (bind _returnvalue_2 (`DecalComponent.CreateDynamicMaterialInstance` (`self.Decal`)))
  (set `self.Decal DMI` _returnvalue_2)
  (bind _returnvalue_3 (`KismetRenderingLibrary.CreateRenderTarget2D` (`KismetMathLibrary.FTrunc` (* (.x _boxextent) 5.0)) (`KismetMathLibrary.FTrunc` (* (.y _boxextent) 5.0)) "RTF_RGBA8" (struct)))
  (bind _output_get (set `SceneCaptureComponent2D.TextureTarget` _returnvalue_3 _scenecapturecomponent2d))
  (set `SceneCaptureComponent.ShowOnlyActors` (`|MakeArray` self :!type "Actor Object Reference") _scenecapturecomponent2d)
  (`MaterialInstanceDynamic.SetTextureParameterValue` (`self.Decal DMI`) "Projection" _output_get))

(fn `UserConstructionScript`)