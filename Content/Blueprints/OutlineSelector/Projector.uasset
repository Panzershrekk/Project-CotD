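; Projector actor that captures its own static mesh into a render target and projects that image through a decal.
; The construction script sizes the decal, the capture's ortho width and a new render target from the mesh bounds.
; The scene capture's show-only list holds just this actor, and its texture feeds the decal's dynamic material as the Projection parameter.
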(event `self.ReceiveBeginPlay`)

(fn `UserConstructionScript`
  (bind _decal (`self.Decal`))
  (bind _scenecapturecomponent2d (`self.SceneCaptureComponent2D`))
  (bind (_origin _boxextent) (`KismetSystemLibrary.GetComponentBounds` (`self.StaticMesh`)))
  (bind _returnvalue (`KismetMathLibrary.FMax` (.x _boxextent) (.y _boxextent)))
  (`DecalsUtils.SetDecalSize` _decal (`KismetMathLibrary.MakeVector` (.x _boxextent) (.y _boxextent) _returnvalue))
  (`SceneComponent.SetWorldScale3D` _decal (1.0 1.0 1.0))
  (`SceneComponent.K2_SetRelativeRotation` _decal (struct :`Pitch` -90.0) false false)
  (set `SceneCaptureComponent2D.OrthoWidth` (* _returnvalue 2.0) (`self.SceneCaptureComponent2D`))
  (bind _returnvalue_2 (`DecalComponent.CreateDynamicMaterialInstance` (`self.Decal`)))
  (set `self.Decal DMI` _returnvalue_2)
  (bind _returnvalue_3 (`KismetRenderingLibrary.CreateRenderTarget2D` (`KismetMathLibrary.FTrunc` (* (.x _boxextent) 5.0)) (`KismetMathLibrary.FTrunc` (* (.y _boxextent) 5.0)) "RTF_RGBA8" (struct)))
  (bind _output_get (set `SceneCaptureComponent2D.TextureTarget` _returnvalue_3 _scenecapturecomponent2d))
  (set `SceneCaptureComponent.ShowOnlyActors` (`|MakeArray` self) _scenecapturecomponent2d)
  (`MaterialInstanceDynamic.SetTextureParameterValue` (`self.Decal DMI`) "Projection" _output_get))