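; Gameplay ability for an unarmed strike that deals damage to the avatar's selected targets.
; On commit it plays the anim instance's CastMontage and waits for a single BattleEvent.ComputeDamage gameplay event.
; That event applies GE_DealDamage to each actor in the instigator's SpellsTargetCopy, resets IsAttacking and ends the ability.
; Ending clears the target list; montage callbacks only print debug text.
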(event `self.K2_ActivateAbility`
  (bind _returnvalue (`self.K2_CommitAbility`))
  (if _returnvalue
    (bind _asbp_template_controllable (cast `/Game/Blueprints/Entities/Controllable/BP_TemplateControllable` (`self.GetAvatarActorFromActorInfo`)))
    (bind _asabp_anim_template (cast `/Game/Animation/ABP_Anim_Template` (`SkeletalMeshComponent.GetAnimInstance` (`Character.Mesh` _asbp_template_controllable))))
    (bind _castmontage (`/Game/Animation/ABP_Anim_Template.CastMontage` _asabp_anim_template))
    (`KismetSystemLibrary.PrintText` (`KismetTextLibrary.Conv_ObjectToText` _castmontage))
    (`AbilityTask_PlayMontageAndWait.CreatePlayMontageAndWaitProxy` "None" _castmontage 1.0 "None" false
      (:`then`
        ;[1 0.03833 0] Specific
        (bind (_asynctaskproxy _payload) (`AbilityTask_WaitGameplayEvent.WaitGameplayEvent` (struct :`TagName` "BattleEvent.ComputeDamage") null true)
          (:`EventReceived`
            (bind _asbp_template_controllable_2 (cast `/Game/Blueprints/Entities/Controllable/BP_TemplateControllable` (`.Instigator` (break `GameplayEventData` _payload)))
              (:`then`
                (for _array_element (`/Game/Blueprints/Entities/Controllable/BP_TemplateControllable.SpellsTargetCopy` _asbp_template_controllable_2)
                  ;[0.6398 0.1102 1] Specific ?
                  (`self.ApplyCustomGameplayEffectToTarget` self (`AbilitySystemBlueprintLibrary.GetAbilitySystemComponent` _array_element) "/Game/GE_GameplayEffect/GE_DealDamage.GE_DealDamage_C"))
                ;[1 0.03833 0] Specific
                (set `/Game/Animation/ABP_Anim_Template.isAttacking` false _asabp_anim_template))
              (:`CastFailed`
                _))
            (`self.K2_EndAbility` :!label _label))))
      (:`OnCompleted`
        (`KismetSystemLibrary.PrintString` "Completed" true true (struct :`R` 1.0 :`G` 0.947948 :`A` 1.0)))
      (:`OnBlendOut`
        (`KismetSystemLibrary.PrintString` "Blended" true true (struct :`R` 1.0 :`G` 0.947948 :`A` 1.0)))
      (:`OnInterrupted`
        (`KismetSystemLibrary.PrintString` "Interrupted" true true (struct :`R` 1.0 :`G` 0.947948 :`A` 1.0)))
      (:`OnCancelled`
        (`KismetSystemLibrary.PrintString` "Cancelled" true true (struct :`R` 1.0 :`G` 0.947948 :`A` 1.0))))
    (else
      (goto _label))))

(event `self.K2_OnEndAbility`
  (params (bWasCancelled :type Boolean))
  (`KismetArrayLibrary.Array_Clear` (`/Game/Blueprints/Entities/Controllable/BP_TemplateControllable.SpellsTargetCopy` (stale `self.K2_ActivateAbility` _asbp_template_controllable)))
  (`KismetSystemLibrary.PrintString` "ClearedTarget" true true (struct :`R` 1.0 :`B` 0.068364 :`A` 1.0)))