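; Base gameplay ability template that casts a spell from a BP_TemplateControllable onto its copied target list.
; After commit, it plays a montage looked up in the anim blueprint and waits for the BattleEvent.AnimProc event; one enum value skips this.
; Projectile spells spawn their actor and apply effects when it finishes, while others apply every effect to each target's COTD ability system immediately.
; Ending the ability clears targets and restores control.
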(event `ApplyEffectToTargets`
  (for _array_element (`self.AbilityTemporarySpell Targets`)
    (for _array_element_2 (`self.EffectsToApply`)
      (bind _ascotdability_system_component (cast `COTDAbilitySystemComponent` (`AbilitySystemBlueprintLibrary.GetAbilitySystemComponent` _array_element)))
      (`/Engine/EditorBlueprintResources/StandardMacros.IsValid` _ascotdability_system_component
        (:`Is Valid`
          (`COTDAbilitySystemComponent.ApplyCustomGameplayEffectToTarget` _ascotdability_system_component self _ascotdability_system_component _array_element_2 0.0)))))
  (`self.K2_EndAbility`))

(event `self.K2_ActivateAbility`
  (bind _montagetoplay (`self.MontageToPlay`))
  (`KismetArrayLibrary.Array_Clear` (`self.AbilityTemporarySpell Targets`))
  (bind _returnvalue (`self.K2_CommitAbility`))
  (if _returnvalue
    (bind _asbp_template_controllable (cast `/Game/Blueprints/Entities/Controllable/BP_TemplateControllable` (`self.GetAvatarActorFromActorInfo`)))
    (set `self.AbilityTemporarySpell Targets` (`/Game/Blueprints/Entities/Controllable/BP_TemplateControllable.SpellsTargetCopy` _asbp_template_controllable))
    (bind _asabp_anim_template (cast `/Game/Animation/ABP_Anim_Template` (`SkeletalMeshComponent.GetAnimInstance` (`Character.Mesh` _asbp_template_controllable))))
    (if (`|EnumEquality` _montagetoplay "NewEnumerator2")
      (`self.ApplyEffectToTargets` :!label _label)
      (else
        (`AbilityTask_PlayMontageAndWait.CreatePlayMontageAndWaitProxy` "None" (`BlueprintMapLibrary.Map_Find` (`/Game/Animation/ABP_Anim_Template.Montages` _asabp_anim_template) _montagetoplay) 1.0 "None" false
          (:`then`
            (bind (_asynctaskproxy _payload) (`AbilityTask_WaitGameplayEvent.WaitGameplayEvent` (struct :`TagName` "BattleEvent.AnimProc") null true)
              (:`EventReceived`
                (bind _spellbeingcast (`/Game/Blueprints/Entities/Controllable/BP_TemplateControllable.SpellBeingCast` _asbp_template_controllable))
                (bind _abilitiesdataasset (`COTDGameplayAbility.AbilitiesDataAsset` _spellbeingcast))
                (if (`AbilitiesDataAsset.IsProjectile` _abilitiesdataasset)
                  (bind (_asynctaskproxy_2 _spawnedactor) (`AbilityTask_SpawnActor.SpawnActor` (struct) (`AbilitiesDataAsset.ProjectileActor` _abilitiesdataasset) null)
                    (:`Success`
                      (bind _asbpproj_base_projectile (cast `/Game/Blueprints/Projectile/BPProj_BaseProjectile` _spawnedactor)
                        (:`then`
                          (add `/Game/Blueprints/Projectile/BPProj_BaseProjectile.OnFinished` _asbpproj_base_projectile (delegate `ApplyEffectToTargets`))
                          (`/Game/Blueprints/Projectile/BPProj_BaseProjectile.Setup` _asbpproj_base_projectile _spellbeingcast 2000.0 (`/Game/Blueprints/Entities/Controllable/BP_TemplateControllable.SpellLocation` _asbp_template_controllable)))
                        (:`CastFailed`
                          (goto _label))))
                    (:`DidNotSpawn`
                      (goto _label)))
                  (else
                    (goto _label)))))))))
    (else
      (`self.K2_EndAbility`))))

(event `self.K2_OnEndAbility`
  (params (bWasCancelled :type Boolean))
  (`KismetArrayLibrary.Array_Clear` (`/Game/Blueprints/Entities/Controllable/BP_TemplateControllable.SpellsTargetCopy` (stale `self.K2_ActivateAbility` _asbp_template_controllable)))
  (set `/Game/Blueprints/Entities/Controllable/BP_TemplateControllable.CanControl` true (stale `self.K2_ActivateAbility` _asbp_template_controllable))
  (`KismetArrayLibrary.Array_Clear` (`self.AbilityTemporarySpell Targets`))
  (`KismetSystemLibrary.PrintString` "ClearedTarget" true true (struct :`R` 1.0 :`B` 0.068364 :`A` 1.0)))